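; MyFPCharacter is a player character Blueprint with modular helmet and vest gear and an inventory screen.
; The construction script sets Mesh as master pose component for HelmetMesh and VestMesh, so both follow the body's animation.
; Pressing Tab creates a new WBP_Inventory, adds it to the viewport, shows the cursor and switches input to UI-only.
; BeginPlay, overlap and Tick are empty, and a Health debug print is unconnected.
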(event EventBeginPlay)

(event Collision|EventActorBeginOverlap
  (params (OtherActor :type Actor%20Object%20Reference)))

(event EventTick
  (params (DeltaSeconds :type Float%20%28single-precision%29)))

(event Input|KeyboardEvents|Tab
  (params (Key :type Key%20Structure :default "None"))
  (bind _returnvalue (Game|GetPlayerController 0))
  (:Pressed
    (bind _returnvalue_2 (UserInterface|CreateWidget "/Game/Assets/WBP_Inventory.WBP_Inventory_C" (Game|GetPlayerController 0)))
    (UserInterface|Viewport|AddtoViewport _returnvalue_2 0)
    (Variables|/Script/Engine.PlayerController|SetbShowMouseCursor _returnvalue true)
    (Input|SetInputModeUIOnly _returnvalue _returnvalue_2 "DoNotLock")))

(fn ConstructionScript
  (Class|SkinnedMeshComponent|SetMasterPoseComponent (Variables|Default|GetHelmetMesh) (Variables|Character|GetMesh) false))